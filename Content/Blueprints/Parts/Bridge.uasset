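; Bridge is a part Blueprint that makes the player's RunCharacter slip while crossing it and introduces the bridge with a tutorial.
; On its first player overlap, BridgeCollider sets the character's Speed and turns Slipping on.
; The first end overlap clears Slipping but leaves Speed unchanged, with a DoOnce guarding each direction.
; TutorialBox shows a TutorialMessages widget on overlap unless RunGameInstance's SeenBridge flag is set, then sets that flag.
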(event OnComponentBeginOverlap(TutorialBox)
  (params (OverlappedComponent :type Primitive%20Component%20Object%20Reference) (OtherActor :type Actor%20Object%20Reference) (OtherComp :type Primitive%20Component%20Object%20Reference) (OtherBodyIndex :type Integer) (bFromSweep :type Boolean) (SweepResult :type Hit%20Result%20Structure%20%28by%20ref%29))
  (bind _asrun_game_instance (Utilities|Casting|CastToRunGameInstance (Game|GetGameInstance)))
  (if (not (Variables|/Game/Blueprints/RunGameInstance.RunGameInstance_C|GetSeenBridge _asrun_game_instance))
    (bind _returnvalue (UserInterface|CreateWidget "/Game/Widgets/TutorialMessages.TutorialMessages_C" (Game|GetPlayerController 0)))
    (Variables|/Game/Widgets/TutorialMessages.TutorialMessages_C|SetMessageToShow _returnvalue 1)
    (UserInterface|Viewport|AddtoViewport _returnvalue 0)
    (bind _asrun_game_instance_2 (Utilities|Casting|CastToRunGameInstance (Game|GetGameInstance)))
    (Variables|/Game/Blueprints/RunGameInstance.RunGameInstance_C|SetSeenBridge _asrun_game_instance_2 true)))

(event OnComponentBeginOverlap(BridgeCollider)
  (params (OverlappedComponent :type Primitive%20Component%20Object%20Reference) (OtherActor :type Actor%20Object%20Reference) (OtherComp :type Primitive%20Component%20Object%20Reference) (OtherBodyIndex :type Integer) (bFromSweep :type Boolean) (SweepResult :type Hit%20Result%20Structure%20%28by%20ref%29))
  (if (== OtherActor (Game|Player|GetPlayerPawn 0))
    (Utilities|FlowControl|DoOnce false
      (:Completed
        (bind _asrun_character (Utilities|Casting|CastToRunCharacter (Game|Player|GetPlayerPawn 0)))
        (Variables|/Game/Blueprints/RunCharacter.RunCharacter_C|Setspeed _asrun_character 35.0)
        (Variables|/Game/Blueprints/RunCharacter.RunCharacter_C|SetSlipping _asrun_character true)))))

(event OnComponentEndOverlap(BridgeCollider)
  (params (OverlappedComponent :type Primitive%20Component%20Object%20Reference) (OtherActor :type Actor%20Object%20Reference) (OtherComp :type Primitive%20Component%20Object%20Reference) (OtherBodyIndex :type Integer))
  (if (== OtherActor (Game|Player|GetPlayerPawn 0))
    (Utilities|FlowControl|DoOnce false
      (:Completed
        (bind _asrun_character (Utilities|Casting|CastToRunCharacter (Game|Player|GetPlayerPawn 0)))
        (Variables|/Game/Blueprints/RunCharacter.RunCharacter_C|SetSlipping _asrun_character false)))))

(fn ConstructionScript)