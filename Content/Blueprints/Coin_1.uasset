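; Coin pickup for a runner game that adds its Value to the player character's Money.
; Sphere overlap by the player pawn credits the money, plays a 2D coin sound at the game instance's SoundVolume and destroys the coin.
; The same overlap shows a TutorialMessages widget once, tracked by the game instance's SeenMoney flag.
; Tick spins the mesh by a fixed step, so its speed depends on frame rate.
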(event OnComponentBeginOverlap(Sphere)
  (params (OverlappedComponent :type Primitive%20Component%20Object%20Reference) (OtherActor :type Actor%20Object%20Reference) (OtherComp :type Primitive%20Component%20Object%20Reference) (OtherBodyIndex :type Integer) (bFromSweep :type Boolean) (SweepResult :type Hit%20Result%20Structure%20%28by%20ref%29))
  (bind _mycharacter (Variables|Default|GetMyCharacter))
  (if (== OtherActor (Game|Player|GetPlayerPawn 0))
    (Utilities|FlowControl|Sequence
      (:then_0
        (Variables|/Game/Blueprints/RunCharacter.RunCharacter_C|Setmoney _mycharacter (+ (Variables|Default|GetValue) (Variables|/Game/Blueprints/RunCharacter.RunCharacter_C|Getmoney _mycharacter)))
        (bind _asrun_game_instance (Utilities|Casting|CastToRunGameInstance (Game|GetGameInstance)))
        (Audio|PlaySound2D "/Game/Audio/Coin.Coin" (Variables|/Game/Blueprints/RunGameInstance.RunGameInstance_C|GetSound%20Volume _asrun_game_instance))
        (Actor|DestroyActor))
      (:then_1
        (bind _asrun_game_instance_2 (Utilities|Casting|CastToRunGameInstance (Game|GetGameInstance)))
        (if (not (Variables|/Game/Blueprints/RunGameInstance.RunGameInstance_C|GetSeenMoney _asrun_game_instance_2))
          (bind _returnvalue (UserInterface|CreateWidget "/Game/Widgets/TutorialMessages.TutorialMessages_C" (Game|GetPlayerController 0)))
          (Variables|/Game/Widgets/TutorialMessages.TutorialMessages_C|SetMessageToShow _returnvalue 6)
          (UserInterface|Viewport|AddtoViewport _returnvalue 0)
          (bind _asrun_game_instance_3 (Utilities|Casting|CastToRunGameInstance (Game|GetGameInstance)))
          (Variables|/Game/Blueprints/RunGameInstance.RunGameInstance_C|SetSeenMoney _asrun_game_instance_3 true))))))

(event EventTick
  (params (DeltaSeconds :type Float%20%28single-precision%29))
  (Transformation|AddLocalRotation (Variables|Default|GetStaticMeshComponent0) "0,10.000000, 0" false false))

(event EventBeginPlay
  ;[1 1 1] Allow HUD to access character variables
  (bind _asrun_character (Utilities|Casting|CastToRunCharacter (Game|GetPlayerCharacter 0)))
  (Variables|Default|SetMyCharacter _asrun_character))

(fn ConstructionScript)