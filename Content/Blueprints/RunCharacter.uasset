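; Player character for a runner game that moves itself forward with swept location offsets, accelerating each tick up to MaxSpeed.
; Input axes strafe it sideways within MaxHorizontal limits, independent of delta time, and actions trigger jump and crouch.
; Any actor overlap subtracts placeholder damage from Health and sets Speed negative, knocking it backward until it re-accelerates.
; It also creates the HUD and a reusable pause menu, swapping input mode, cursor and visibility.
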(event Custom|Resume
  (Input|SetInputModeGameOnly (Variables|Default|GetcontrollerRef))
  (Widget|SetVisibility (Variables|Default|GetpauseMenuRef) "Collapsed")
  (Game|SetGamePaused false)
  (Variables|/Script/Engine.PlayerController|SetbShowMouseCursor (Variables|Default|GetcontrollerRef) false)
  (Widget|SetVisibility (Variables|Default|GethudRef) "Visible"))

(event EventBeginPlay
  (bind _returnvalue (Game|GetPlayerController 0))
  (bind _returnvalue_2 (UserInterface|CreateWidget "/Game/Widgets/HUD.HUD_C"))
  (bind _output_get (Variables|Default|SethudRef _returnvalue_2))
  (UserInterface|Viewport|AddtoViewport _output_get 0)
  (bind _output_get_2 (Variables|Default|SetcontrollerRef _returnvalue))
  (Input|SetInputModeGameOnly _output_get_2)
  (Input|EnableInput _returnvalue))

(event Collision|EventActorBeginOverlap
  (params (OtherActor :type Actor%20Object%20Reference))
  (Variables|Default|Sethealth (- (Variables|Default|Gethealth) 1e+01))
  (Variables|Default|Setspeed -1e+01))

(event EventTick
  (params (DeltaSeconds :type Float%20%28single-precision%29))
  (Transformation|SetActorLocation (+ (* "8.000000,0.000000,1.000000" (* DeltaSeconds (Variables|Default|Getspeed))) (Transformation|GetActorLocation)) true false)
  (if (>= (Variables|Default|Getspeed) 2e+01)
    (if (>= (Variables|Default|Getspeed) (Variables|Default|GetmaxSpeed))
      (Variables|Default|Setspeed (Variables|Default|GetmaxSpeed))
      (else
        (Variables|Default|Setspeed (+ (Variables|Default|Getacceleration) (Variables|Default|Getspeed)))))
    (else
      (Variables|Default|Setspeed (+ (* (Variables|Default|Getacceleration) 1.0) (Variables|Default|Getspeed))))))

(event Input|ActionEvents|InputActionPause
  (params (Key :type Key%20Structure :default "AnyKey"))
  (:Pressed
    (Utilities|IsValid (Variables|Default|GetpauseMenuRef)
      (:Is%20Valid
        _)
      (:Is%20Not%20Valid
        (bind _returnvalue (UserInterface|CreateWidget "/Game/Widgets/PauseMenu.PauseMenu_C"))
        (bind _output_get (Variables|Default|SetpauseMenuRef _returnvalue))
        (UserInterface|Viewport|AddtoViewport _output_get 0)
        (EventDispatchers|BindEventtoOnResume (Variables|Default|GetpauseMenuRef) (delegate Custom|Resume))))
    (Input|SetInputModeUIOnly (Variables|Default|GetcontrollerRef) (Variables|Default|GetpauseMenuRef) false)
    (Variables|/Script/Engine.PlayerController|SetbShowMouseCursor (Variables|Default|GetcontrollerRef) true)
    (Widget|SetVisibility (Variables|Default|GetpauseMenuRef) "Visible")
    (Widget|SetVisibility (Variables|Default|GethudRef) "Collapsed")
    (Game|SetGamePaused true)))

(event Input|ActionEvents|InputActionDuck
  (params (Key :type Key%20Structure :default "AnyKey"))
  (:Pressed
    (Character|Crouch))
  (:Released
    (Character|UnCrouch)))

(event Input|ActionEvents|InputActionJump
  (params (Key :type Key%20Structure :default "AnyKey"))
  (:Pressed
    (Character|Jump)))

(event Input|AxisEvents|InputAxisMoveLeft
  (params (AxisValue :type Float%20%28single-precision%29))
  (bind _returnvalue (Transformation|GetActorLocation))
  (bind _horizontalspeed (Variables|Default|GethorizontalSpeed))
  (bind _returnvalue_2 (* AxisValue _horizontalspeed))
  (bind _returnvalue_3 (* "0,-1.000000, 0" _returnvalue_2))
  (bind _returnvalue_4 (+ _returnvalue_3 _returnvalue))
  (bind (_x _y _z) (Math|Vector|BreakVector _returnvalue_4))
  (Transformation|SetActorLocation (Math|Vector|MakeVector _x (Math|Float|Max(Float) _y (* -1 (Variables|Default|GetmaxHorizontal))) _z) true false))

(event Input|AxisEvents|InputAxisMoveRight
  (params (AxisValue :type Float%20%28single-precision%29))
  (bind _returnvalue (Transformation|GetActorLocation))
  (bind _horizontalspeed (Variables|Default|GethorizontalSpeed))
  (bind _returnvalue_2 (* AxisValue _horizontalspeed))
  (bind _returnvalue_3 (* "0,1.000000, 0" _returnvalue_2))
  (bind _returnvalue_4 (+ _returnvalue_3 _returnvalue))
  (bind (_x _y _z) (Math|Vector|BreakVector _returnvalue_4))
  (Transformation|SetActorLocation (Math|Vector|MakeVector _x (Math|Float|Min(Float) _y (Variables|Default|GetmaxHorizontal)) _z) true false))

(fn ConstructionScript)