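; MMGameMode is a game mode, likely for the main menu, that applies saved audio volumes to level sounds when play begins.
; On BeginPlay it finds every AmbientSound actor and reads volumes from the RunGameInstance.
; Audio components tagged "music" get the music volume multiplier, and all others get the sound volume multiplier.
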(event EventBeginPlay
  (bind _outactors (Actor|GetAllActorsOfClass "/Script/Engine.AmbientSound"))
  (for _array_element _outactors
    (bind _asrun_game_instance (Utilities|Casting|CastToRunGameInstance (Game|GetGameInstance)))
    (if (Components|ComponentHasTag (Variables|/Script/Engine.AmbientSound|GetAudioComponent _array_element) "music")
      (Audio|Components|Audio|SetVolumeMultiplier (Variables|/Script/Engine.AmbientSound|GetAudioComponent _array_element) (Variables|/Game/Blueprints/RunGameInstance.RunGameInstance_C|GetMusic%20Volume _asrun_game_instance) :!class /Script/Engine.AudioComponent)
      (else
        (Audio|Components|Audio|SetVolumeMultiplier (Variables|/Script/Engine.AmbientSound|GetAudioComponent _array_element) (Variables|/Game/Blueprints/RunGameInstance.RunGameInstance_C|GetSound%20Volume _asrun_game_instance) :!class /Script/Engine.AudioComponent)))))

(event EventTick
  (params (DeltaSeconds :type Float%20%28single-precision%29)))

(fn ConstructionScript)