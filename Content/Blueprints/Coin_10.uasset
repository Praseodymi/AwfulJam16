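; Coin pickup actor that adds its Value to the player's money when collected.
; On BeginPlay it caches the player character as RunCharacter.
; When the player pawn overlaps the Sphere, it increases that character's Money, plays a 2D coin sound and destroys itself.
; Tick spins the static mesh by a fixed step each frame, so rotation speed depends on frame rate.
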(event OnComponentBeginOverlap(Sphere)
  (params (OverlappedComponent :type Primitive%20Component%20Object%20Reference) (OtherActor :type Actor%20Object%20Reference) (OtherComp :type Primitive%20Component%20Object%20Reference) (OtherBodyIndex :type Integer) (bFromSweep :type Boolean) (SweepResult :type Hit%20Result%20Structure%20%28by%20ref%29))
  (bind _mycharacter (Variables|Default|GetMyCharacter))
  (if (== OtherActor (Game|Player|GetPlayerPawn 0))
    (Variables|/Game/Blueprints/RunCharacter.RunCharacter_C|Setmoney _mycharacter (+ (Variables|Default|GetValue) (Variables|/Game/Blueprints/RunCharacter.RunCharacter_C|Getmoney _mycharacter)))
    (Audio|PlaySound2D "/Game/Audio/Coin.Coin")
    (Actor|DestroyActor)))

(event Collision|EventActorBeginOverlap
  (params (OtherActor :type Actor%20Object%20Reference)))

(event EventTick
  (params (DeltaSeconds :type Float%20%28single-precision%29))
  (Transformation|AddLocalRotation (Variables|Default|GetStaticMeshComponent0) "0,10.000000, 0" false false))

(event EventBeginPlay
  ;[1 1 1] Allow HUD to access character variables
  (bind _asrun_character (Utilities|Casting|CastToRunCharacter (Game|GetPlayerCharacter 0)))
  (Variables|Default|SetMyCharacter _asrun_character))

(fn ConstructionScript)