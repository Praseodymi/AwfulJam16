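; LevelCreator is an actor that builds a randomized level from tile pieces on BeginPlay, starting at its own transform.
; It spawns random LevelPieces in a loop, using a shifted random index intended to avoid repeating the previous piece.
; Each piece advances the next spawn location by LevelPieceOffset scaled by that piece's TileSize entry.
; Valid spawned actors are stored in LevelArray.
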(event EventBeginPlay
  (bind _levelpieces (Variables|Default|GetLevelPieces))
  (bind _returnvalue (Utilities|Array|Length _levelpieces))
  (bind _returnvalue_2 (- _returnvalue 1))
  (Variables|Default|SetNextTransform (Transformation|GetActorTransform self))
  (for _index (range 0 (Variables|Default|GetLevelTileCount))
    (if (== _index 0)
      (Variables|Default|SetRandomInt (Math|Random|RandomIntegerinRange 0 _returnvalue_2))
      (else
        (bind _output_get (Variables|Default|SetTempRandomInt (Math|Random|RandomIntegerinRange 0 (- _returnvalue_2 1))))
        (if (< _output_get (Variables|Default|GetRandomInt))
          _
          (else
            (bind _result (Math|Integer|IncrementInt (Variables|Default|GetTempRandomInt))
              (:%20%20
                _))))
        (Variables|Default|SetRandomInt _result)))
    (bind _returnvalue_3 (Game|SpawnActorfromClass (Utilities|Array|Get(acopy) _levelpieces (Variables|Default|GetRandomInt)) (Variables|Default|GetNextTransform) "AlwaysSpawn" self 0))
    (Variables|Default|SetNextTransform (Math|Transform|MakeTransform (+ (* (Variables|Default|GetLevelPieceOffset) (Utilities|Array|Get(acopy) (Variables|Default|GetTileSize) (Variables|Default|GetRandomInt))) (.Location (Math|Transform|BreakTransform (Variables|Default|GetNextTransform)))) (.Rotation (Math|Transform|BreakTransform (Variables|Default|GetNextTransform))) (.Scale (Math|Transform|BreakTransform (Variables|Default|GetNextTransform)))))
    (if (Utilities|IsValid _returnvalue_3)
      (Utilities|Array|Add (Variables|Default|GetLevelArray) _returnvalue_3))))

(event Collision|EventActorBeginOverlap
  (params (OtherActor :type Actor%20Object%20Reference)))

(event EventTick
  (params (DeltaSeconds :type Float%20%28single-precision%29)))

(fn ConstructionScript)