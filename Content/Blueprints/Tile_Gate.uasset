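; Gate tile Blueprint whose two doors swing open the first time anything triggers its Box overlap.
; A DoOnce plays hit and creak sounds at the world origin, then starts the Open timeline.
; The timeline lerps GateA and GateB relative yaw in opposite directions, scaled by SharedRoot's world X scale, so negative scale flips the swing.
; The Box is destroyed when the timeline finishes.
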(event OnComponentBeginOverlap(Box)
  (params (OverlappedComponent :type Primitive%20Component%20Object%20Reference) (OtherActor :type Actor%20Object%20Reference) (OtherComp :type Primitive%20Component%20Object%20Reference) (OtherBodyIndex :type Integer) (bFromSweep :type Boolean) (SweepResult :type Hit%20Result%20Structure%20%28by%20ref%29))
  (bind _sharedroot (Variables|Default|GetSharedRoot))
  (bind _returnvalue (Transformation|GetWorldScale _sharedroot))
  (bind _x (Math|Vector|BreakVector _returnvalue))
  (bind _returnvalue_2 (* _x -9e+01))
  (bind _returnvalue_3 (Math|Rotator|MakeRotator 0.0 0.0 _returnvalue_2))
  (Utilities|FlowControl|DoOnce false
    (:Completed
      (Audio|SpawnSoundatLocation "/Game/Audio/GateHit.GateHit" "0, 0, 0")
      (Audio|PlaySoundatLocation "/Game/Audio/GateCreak.GateCreak" "0, 0, 0")
      (bind _newtrack_0 (Timeline|Open PlayFromStart)
        (:Update
          (Transformation|SetRelativeRotation (Variables|Default|GetGateA) (Math|Rotator|Lerp(Rotator) "0, 0, 0" _returnvalue_3 _newtrack_0) false false)
          (Transformation|SetRelativeRotation (Variables|Default|GetGateB) (Math|Rotator|Lerp(Rotator) (Math|Rotator|MakeRotator 0.0 0.0 (* _x -1.8e+02)) _returnvalue_3 _newtrack_0) false false))
        (:Finished
          (Components|DestroyComponent (Variables|Default|GetBox)))))))

(fn ConstructionScript)